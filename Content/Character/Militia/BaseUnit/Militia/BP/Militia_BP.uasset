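; Militia base unit character that spawns with an AK rifle in hand.
; On BeginPlay it caches its MilitiaAnim instance, spawns AK_BP onto the mesh's weapon socket, and attaches OpenFirePoint to the rifle's firing socket.
; Each Tick it writes mesh velocity and the anim instance's forward and right move values into up vectors read from MoveDirection, AnimMoveForward and AnimMoveRight, without applying them back.
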(event `self.ReceiveBeginPlay`
  (bind _asmilitia_anim (cast `/Game/Character/Militia/BaseUnit/Militia/Anim/MilitiaAnim` (`SkeletalMeshComponent.GetAnimInstance` (`self.Mesh`))))
  (set `self.As Militia Anim` _asmilitia_anim)
  ;[1 1 1] Weapon Attach
  (bind _returnvalue (`|SpawnActorFromClass` "/Game/Weapon/AK_BP.AK_BP_C" (`KismetMathLibrary.MakeTransform` (0.0 0.0 0.0)) "Undefined" "OverrideRootScale" null null))
  (bind _output_get (set `self.AK_Instance` _returnvalue))
  (`self.K2_AttachToComponent` _output_get (`self.Mesh`) (`self.WeaponSlot`) "SnapToTarget" "SnapToTarget" "SnapToTarget" true)
  ;[1 1 1] OpenFirePoint Attach
  (`SceneComponent.K2_AttachToComponent` (`self.OpenFirePoint`) (`/Game/Weapon/WeaponBase_BP.Weapon_SK` _output_get) (`self.OpenFireSlot`) "SnapToTarget" "SnapToTarget" "KeepWorld" true))

(event `self.ReceiveTick`
  (params (DeltaSeconds :type "Float (single-precision)"))
  (bind (_x _y) (`KismetMathLibrary.BreakVector3f` (`SceneComponent.GetComponentVelocity` (`self.Mesh`))))
  (`KismetMathLibrary.Vector_Set` (`SceneComponent.GetUpVector` (`self.MoveDirection`)) _x _y)
  (bind _asmilitia_anim (cast `/Game/Character/Militia/BaseUnit/Militia/Anim/MilitiaAnim` (`SkeletalMeshComponent.GetAnimInstance` (`self.Mesh`))))
  (`KismetMathLibrary.Vector_Set` (`SceneComponent.GetUpVector` (`self.AnimMoveRight`)) 0.0 (`/Game/Character/Militia/BaseUnit/Militia/Anim/MilitiaAnim.MoveRight_AB` _asmilitia_anim))
  (`KismetMathLibrary.Vector_Set` (`SceneComponent.GetUpVector` (`self.AnimMoveForward`)) (`/Game/Character/Militia/BaseUnit/Militia/Anim/MilitiaAnim.MoveForward_AB` _asmilitia_anim)))

(fn `UserConstructionScript`
  (`parent.UserConstructionScript`))