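; Mob1 monster Blueprint that pins its body-part components to the skeleton of a mob character.
; The construction script runs the parent's, then attaches the head, shoulder, elbow, hand, chest and tail components to same-named Mesh sockets.
; Each attachment snaps to the socket's location while keeping world rotation and scale.
; The event graph holds only empty stubs, including Tick and a click event on TraceShowCharacterInformation, so it adds no runtime logic.
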(event `self.ReceiveTick`
  (params (DeltaSeconds :type "Float (single-precision)")))

(event `self.TraceShowCharacterInformation.OnClicked`
  (params (TouchedComponent :type "PrimitiveComponent Object Reference") (ButtonPressed :type "Key Structure")))

(fn `UserConstructionScript`
  (bind _mesh (`self.Mesh`))
  (bind _mesh_2 (`self.Mesh`))
  (`parent.UserConstructionScript`)
  (`SceneComponent.K2_AttachToComponent` (`self.Head`) _mesh "Head" "SnapToTarget" "KeepWorld" "KeepWorld" true)
  (`SceneComponent.K2_AttachToComponent` (`self.LShoulder`) _mesh "LShoulder" "SnapToTarget" "KeepWorld" "KeepWorld" true)
  (`SceneComponent.K2_AttachToComponent` (`self.RShoulder`) _mesh "RShoulder" "SnapToTarget" "KeepWorld" "KeepWorld" true)
  (`SceneComponent.K2_AttachToComponent` (`self.LElbow`) _mesh "LElbow" "SnapToTarget" "KeepWorld" "KeepWorld" true)
  (`SceneComponent.K2_AttachToComponent` (`self.RElbow`) _mesh "RElbow" "SnapToTarget" "KeepWorld" "KeepWorld" true)
  (`SceneComponent.K2_AttachToComponent` (`self.LHand`) _mesh_2 "LHand" "SnapToTarget" "KeepWorld" "KeepWorld" true)
  (`SceneComponent.K2_AttachToComponent` (`self.RHand`) _mesh_2 "RHand" "SnapToTarget" "KeepWorld" "KeepWorld" true)
  (`SceneComponent.K2_AttachToComponent` (`self.Chest`) _mesh_2 "Chest" "SnapToTarget" "KeepWorld" "KeepWorld" true)
  (`SceneComponent.K2_AttachToComponent` (`self.Tail`) _mesh_2 "Tail" "SnapToTarget" "KeepWorld" "KeepWorld" true))